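; Spawner actor in the MachineLearning folder that respawns a batch of BP_AIBase targets on demand.
; Its spawnTargets_Event destroys every tracked target, then spawns NumberOfTargets new ones, adding each to SpawnedTargets without clearing old entries.
; Each target lands at a random XY offset within MaxDistanceToSpawn on each axis at the spawner's height, with collision adjusted but spawning guaranteed.
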(event Custom|spawnTargets_Event
  (bind _maxdistancetospawn (Variables|Default|GetmaxDistanceToSpawn))
  (bind _returnvalue (* _maxdistancetospawn -1.0))
  (bind _returnvalue_2 (Math|Random|RandomFloatinRange _returnvalue _maxdistancetospawn))
  (for _array_element (Variables|Default|GetspawnedTargets)
    (Actor|DestroyActor _array_element))
  (Variables|Default|SetspawnCount 0)
  (while (< (Variables|Default|GetspawnCount) (Variables|Default|GetnumberOfTargets))
    (Math|Integer|IncrementInt (Variables|Default|GetspawnCount)
      (:%20%20
        (bind _returnvalue_3 (Game|SpawnActorfromClass "/Game/FirstPersonBP/Blueprints/BP_AIBase.BP_AIBase_C" (Math|Transform|MakeTransform (+ (Transformation|GetActorLocation) (Math|Vector|MakeVector _returnvalue_2 _returnvalue_2 0.0))) "AdjustIfPossibleButAlwaysSpawn" 0 0))
        (Utilities|Array|Add (Variables|Default|GetspawnedTargets) _returnvalue_3)))))

(event Collision|EventActorBeginOverlap
  (params (OtherActor :type Actor%20Object%20Reference)))

(event EventTick
  (params (DeltaSeconds :type Float%20%28single-precision%29)))

(fn ConstructionScript)